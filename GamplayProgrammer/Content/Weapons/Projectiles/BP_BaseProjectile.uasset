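; Base projectile Blueprint that deals damage to the actors it hits.
; The CustomProjectileHit event records each actor in ListOfAffectedActors, so the same actor is never processed twice by one projectile.
; It skips the owning character unless self-damage is allowed, then passes the projectile's damage to the target through an ILoseHealth interface message.
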(event EventCustomProjectileHit
  (params (OtherActor :type Actor%20Object%20Reference))
  ;[1 1 1] Hit actors
  ;;[1 1 1] We have to check this to avoid hitting the same actor twice
  (if (not (Utilities|Array|ContainsItem (Variables|Default|GetListOfAffectedActors) OtherActor))
    (Utilities|Array|AddUnique (Variables|Default|GetListOfAffectedActors) OtherActor)
    ;;[1 1 1] Check if can hurt ourselfs
    (bind _returnvalue (Class|BaseProjectile|GetBaseChOwner))
    (bind _returnvalue_2 (Class|BaseProjectile|CheckCanSelfDamage))
    (if (or _returnvalue_2 (!= _returnvalue OtherActor))
      (bind _returnvalue_3 (Class|BaseProjectile|GetDamage))
      (Class|IHealth|ILoseHealth(Message) OtherActor _returnvalue_3))))

(fn ConstructionScript)